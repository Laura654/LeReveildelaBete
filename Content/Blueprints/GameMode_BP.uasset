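; Game mode for a card game where left/right choices affect per-god gauges and gameplay tags.
; PrepareCards splits data table rows into an available pool and tag-locked groups, which effect tags add or remove.
; ApplyEffect updates gauges, handles replay and menu tags, then plays the specified next card, game-over card or a random non-repeating one.
; BeginPlay, UpdateValue, CardSelected and StartGameOverSequence events have empty bodies here.
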(event `self.ReceiveBeginPlay`)

(event `UpdateValue`
  (params (God :type "/Game/Blueprints/E_Gods Enum" :default "NewEnumerator0") (Modifier :type Integer)))

(event `CardSelected`
  (params (`IsLeftSelected?` :type Boolean)))

(event `StartGameOverSequence`
  (params (God :type "/Game/Blueprints/E_Gods Enum" :default "NewEnumerator0") (`PositiveOverFlow?` :type Boolean)))

(fn `AddCardsInPool`
  (params (Tag :type "GameplayTag Structure"))
  (for _array_element (break `/Game/Blueprints/NameArray_Struct` (`BlueprintMapLibrary.Map_Find` (`self.CardsByTags`) Tag))
    (`KismetArrayLibrary.Array_AddUnique` (`self.AvailableCardsPool`) _array_element)))

(fn `ApplyEffect`
  (params (Effect :type "/Game/Blueprints/GameEffect_Struct Structure"))
  (locals (NextCard :type "DataTableRowHandle Structure"))
  (bind (_nextcard_datatable _nextcard_rowname) (break `DataTableRowHandle` (`local.NextCard`)))
  (set `local.NextCard` Effect_Nextcardtoplay_21_6185EF644A80AFE7B8677F9A17DC3009)
  (for _array_element Effect_EffectsOnGauge_9_69A713C84D69D8E56640859654B384EB
    (`self.UpdateValue` (break `/Game/Blueprints/GodValue_struct` _array_element) (`.EffectValue_6_99A7F8FE4D6B85A9B14F9C9A4616B809` (break `/Game/Blueprints/GodValue_struct` _array_element)))
    (if (`self.bIsGameOver?`)
      (set `local.NextCard` (`self.GameOverCard`))))
  (for _array_element_2 Effect_TagstoAdd_14_E923EF804B1862BDB90C7AB0EE4A08D2
    (`BlueprintGameplayTagLibrary.AddGameplayTag` (`self.GameplaytagContainer`) _array_element_2)
    (if (== _array_element_2 (struct :`TagName` "Rejouer"))
      (`GameplayStatics.OpenLevelBySoftObjectPtr` "/Game/Maps/Game.Game")
      (elif (== _array_element_2 (struct :`TagName` "MenuPrincipal"))
        (`GameplayStatics.OpenLevelBySoftObjectPtr` "/Game/Maps/MainMenu.MainMenu")
        (else
          (`self.AddCardsInPool` _array_element_2)))))
  (for _array_element_3 Effect_TagstoRemove_16_85F2831242A70474DFC8EC97CF6A9793
    (`BlueprintGameplayTagLibrary.RemoveGameplayTag` (`self.GameplaytagContainer`) _array_element_3)
    (`self.RemoveCardsFromPool` _array_element_3))
  (for _array_element_4 Effect_CardsToRemove_25_007EE42C46292A85EAF4CE8054FD3AC1
    (`KismetArrayLibrary.Array_RemoveItem` (`self.AvailableCardsPool`) (`.RowName` (break `DataTableRowHandle` _array_element_4)))
    (`KismetSystemLibrary.PrintString` (`KismetStringLibrary.Concat_StrStr` "Remove : " (`KismetStringLibrary.Conv_NameToString` (`.RowName` (break `DataTableRowHandle` _array_element_4))))))
  (`/Engine/EditorBlueprintResources/StandardMacros.IsValid` _nextcard_datatable
    (:`Is Valid`
      (bind _returnvalue (`|GetDataTableRow` _nextcard_datatable _nextcard_rowname)
        (:`then`
          (`self.SetNextCard` _returnvalue _nextcard_rowname))
        (:`RowNotFound`
          (if (not (`self.bIsGameOver?`)) :!label _label
            (`self.SelectRandomCard`)))))
    (:`Is Not Valid`
      (goto _label))))

(fn `GetValue`
  (params (God :type "/Game/Blueprints/E_Gods Enum (by ref)"))
  (returns (Value :type Integer))
  (return (`BlueprintMapLibrary.Map_Find` (`self.CurrentGaugeValues`) God)))

(fn `GetValueAsRatio`
  (params (God :type "/Game/Blueprints/E_Gods Enum (by ref)"))
  (returns (Ratio :type "Float (double-precision)"))
  (return (`KismetMathLibrary.FClamp` (/ (`KismetMathLibrary.Conv_IntToDouble` (`self.GetValue` God)) (`KismetMathLibrary.Conv_IntToDouble` (`self.MaxGaugeValue`))))))

(fn `PrepareCards`
  (locals (CardData :type "/Game/Blueprints/Card_Struct Structure") (CardRowName :type Name) (TmpArray :type "Array of Name"))
  (bind _outrownames (`DataTableFunctionLibrary.GetDataTableRowNames` (`self.AllCardDT`)))
  (for _array_element _outrownames
    (bind _output_get (set `local.CardRowName` _array_element))
    (bind _returnvalue (`|GetDataTableRow` (`self.AllCardDT`) _output_get)
      (:`then`
        (bind _output_get_2 (set `local.CardData` _returnvalue))
        (if (`BlueprintGameplayTagLibrary.IsGameplayTagValid` (break `/Game/Blueprints/LockCondition_Struct` (break `/Game/Blueprints/Card_Struct` _output_get_2)))
          (bind _output_get_3 (set `local.TmpArray` (break `/Game/Blueprints/NameArray_Struct` (`BlueprintMapLibrary.Map_Find` (`self.CardsByTags`) (break `/Game/Blueprints/LockCondition_Struct` (break `/Game/Blueprints/Card_Struct` _output_get_2))))))
          (`KismetArrayLibrary.Array_AddUnique` _output_get_3 (`local.CardRowName`))
          (`BlueprintMapLibrary.Map_Add` (`self.CardsByTags`) (break `/Game/Blueprints/LockCondition_Struct` (break `/Game/Blueprints/Card_Struct` _output_get_2)) (make `/Game/Blueprints/NameArray_Struct` (`local.TmpArray`)))
          (else
            (`KismetArrayLibrary.Array_AddUnique` (`self.AvailableCardsPool`) (`local.CardRowName`))))))))

(fn `RemoveCardsFromPool`
  (params (Tag :type "GameplayTag Structure (by ref)"))
  (for _array_element (break `/Game/Blueprints/NameArray_Struct` (`BlueprintMapLibrary.Map_Find` (`self.CardsByTags`) Tag))
    (`KismetArrayLibrary.Array_RemoveItem` (`self.AvailableCardsPool`) _array_element)))

(fn `SelectRandomCard`
  (locals (NextRowName :type Name))
  (bind _nextrowname (`local.NextRowName`))
  (if (== (`KismetArrayLibrary.Array_Length` (`self.AvailableCardsPool`)) 0)
    (`KismetSystemLibrary.PrintString` "Problem ! No more available cards !" true true (struct :`R` 1.0 :`A` 1.0) 10.0)
    (else
      (bind _output_get (set `local.NextRowName` (`KismetArrayLibrary.Array_Random` (`self.AvailableCardsPool`)) :!label _label))
      (if (== _output_get (`self.CurrentCardRowName`))
        (`KismetSystemLibrary.PrintString` "Same card" true true (struct :`R` 0.822917 :`G` 0.310237 :`A` 1.0) 5.0)
        (goto _label)
        (else
          (bind _returnvalue (`|GetDataTableRow` (`self.AllCardDT`) _nextrowname)
            (:`then`
              (`self.SetNextCard` _returnvalue _nextrowname))
            (:`RowNotFound`
              (`KismetSystemLibrary.PrintString` "PROBLEM !" true true (struct :`R` 1.0 :`A` 1.0) 10.0))))))))

(fn `SetNextCard`
  (params (Card :type "/Game/Blueprints/Card_Struct Structure") (RowName :type Name))
  (bind (_currentcard_lockcondition _currentcard_onetimeusage) (break `/Game/Blueprints/Card_Struct` (`self.CurrentCard`)))
  (if (and (!= (`self.CurrentCardRowName`) "None") _currentcard_onetimeusage)
    (`KismetArrayLibrary.Array_RemoveItem` (`self.AvailableCardsPool`) (`self.CurrentCardRowName`)))
  (bind _output_get (set `self.CurrentCard` Card))
  (set `self.CurrentCardRowName` RowName)
  (`self.OnNewCard` _output_get))

(fn `UserConstructionScript`)